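; SpawnBox is an actor that rains Boulder actors at random points inside its Box component for a limited time once activated.
; Activate sets the active flag and opens a ten-second spawn window.
; Tick counts down both the window and a spawn cooldown, spawning a boulder every half second while the window lasts.
; The active flag is never cleared here, so the expired window timer alone stops spawning.
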(event EventBeginPlay)

(event EventActorBeginOverlap
  (params (OtherActor :type Actor%20Object%20Reference)))

(event EventTick
  (params (DeltaSeconds :type Float%20%28single-precision%29))
  (bind _box (Variables|Default|GetBox))
  (bind (_origin _boxextent) (Collision|GetComponentBounds _box))
  (Variables|Default|SetTill%20NextSpawn (- (Variables|Default|GetTill%20NextSpawn) DeltaSeconds))
  (bind _output_get (Variables|Default|SetSpawnning (- (Variables|Default|GetSpawnning) DeltaSeconds)))
  (if (Math|Boolean|ANDBoolean (Variables|Default|GetIsAcvite) (> 0.0 (Variables|Default|GetTill%20NextSpawn)) (> _output_get 0.0))
    (Game|SpawnActorfromClass "/Game/Blueprints/Boulder.Boulder_C" (Math|Conversions|ToTransform(Vector) (Math|Random|RandomPointinBoundingBox _origin _boxextent)) "AdjustIfPossibleButAlwaysSpawn" 0 0)
    (Variables|Default|SetTill%20NextSpawn 0.5)))

(fn ConstructionScript)

(fn Activate
  (Variables|Default|SetIsAcvite true)
  (Variables|Default|SetSpawnning 1e+01))