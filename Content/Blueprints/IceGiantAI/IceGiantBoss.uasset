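; Ice giant boss that moves its focus among fire pits and throws timed tantrums.
; On BeginPlay it caches the fire pits and center spot and targets the nearest burning pit; NextNode pauses that pit's fire and follows its NextPit link.
; Tantrum starts a Tick-driven countdown and activates a SpawnBox, then pauses all pits when called after expiry.
; CheckTheTraps reports whether any pit is unlit.
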(event EventBeginPlay
  (bind _outactors (Actor|GetAllActorsOfClass "/Game/Blueprints/FirePit.FirePit_C"))
  (Variables|Default|SetFirePit _outactors)
  (CallFunction|GetClosestFirePit)
  (bind _outactors_2 (Actor|GetAllActorsOfClass "/Game/Blueprints/CenterSpot.CenterSpot_C"))
  (Variables|Default|SetcenterSpot (Utilities|Array|Get(acopy) _outactors_2)))

(event EventActorBeginOverlap
  (params (OtherActor :type Actor%20Object%20Reference)))

(event EventTick
  (params (DeltaSeconds :type Float%20%28single-precision%29))
  (Variables|Default|SetTantrumTimer (- (Variables|Default|GetTantrumTimer) DeltaSeconds)))

(fn ConstructionScript)

(fn GetClosestFirePit
  (bind _firepit (Variables|Default|GetFirePit))
  (for (_array_element _array_index) _firepit
    (if (Variables|/Game/Blueprints/FirePit.FirePit_C|GetOnFire _array_element)
      (if (< (Transformation|GetDistanceTo _array_element) (LocalVariables|GetSmallest))
        (LocalVariables|SetSmallest (Transformation|GetDistanceTo _array_element))
        (LocalVariables|SetIndex _array_index))))
  (Variables|Default|SetCurrentPit (Utilities|Array|Get(acopy) _firepit (LocalVariables|GetIndex))))

(fn NextNode
  (if (Variables|/Game/Blueprints/FirePit.FirePit_C|GetOnFire (Variables|Default|GetCurrentPit))
    (Default|PauseFire (Variables|Default|GetCurrentPit)))
  (Variables|Default|SetCurrentPit (Variables|/Game/Blueprints/FirePit.FirePit_C|GetNextPit (Variables|Default|GetCurrentPit))))

(fn Tantrum
  (if (Variables|Default|GetAttackingPlayer)
    (if (< (Variables|Default|GetTantrumTimer) 0.0)
      (Variables|Default|SetAttackingPlayer false)
      (for _array_element (Variables|Default|GetFirePit)
        (Default|PauseFire _array_element)))
    (else
      (Variables|Default|SetAttackingPlayer true)
      (Variables|Default|SetTantrumTimer 1e+01)
      (bind _outactors (Actor|GetAllActorsOfClass "/Game/Blueprints/SpawnBox.SpawnBox_C"))
      (Default|Activate (Utilities|Array|Get(acopy) _outactors)))))

(fn ChecktheTraps
  (for _array_element (Variables|Default|GetFirePit)
    (if (not (Variables|/Game/Blueprints/FirePit.FirePit_C|GetOnFire _array_element))
      (return true)))
  (return false))