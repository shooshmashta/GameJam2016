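; StartCheck is a behavior tree node that syncs the Ice Giant boss's state to the blackboard on each AI tick.
; It takes the first IceGiantBoss in the level, runs its trap check for ShieldActive, and writes state flags, pit, center, player and distance keys.
; It then restarts the FrostAi controller's brain logic every tick; branches gating this on shield and distance are disconnected.
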(event EventTick
  (params (OwnerActor :type Actor%20Object%20Reference) (DeltaSeconds :type Float%20%28single-precision%29)))

(event EventReceiveTickAI
  (params (OwnerController :type AI%20Controller%20Object%20Reference) (ControlledPawn :type Pawn%20Object%20Reference) (DeltaSeconds :type Float%20%28single-precision%29))
  (bind _returnvalue (Game|GetPlayerCharacter 0))
  (bind _outactors (Actor|GetAllActorsOfClass "/Game/Blueprints/IceGiantAI/IceGiantBoss.IceGiantBoss_C"))
  (bind _output_get (Variables|Default|SetBos (Utilities|Array|Get(acopy) _outactors)))
  (bind _notallfiring (Default|ChecktheTraps _output_get))
  (Class|BTFunctionLibrary|SetBlackboardValueasBool (Variables|Default|GetIsActive) (Variables|/Game/Blueprints/IceGiantAI/IceGiantBoss.IceGiantBoss_C|GetIsActive _output_get))
  (Class|BTFunctionLibrary|SetBlackboardValueasBool (Variables|Default|GetAttackingPlayer) (Variables|/Game/Blueprints/IceGiantAI/IceGiantBoss.IceGiantBoss_C|GetAttackingPlayer _output_get))
  (Class|BTFunctionLibrary|SetBlackboardValueasBool (Variables|Default|GetShieldActive) _notallfiring)
  (Class|BTFunctionLibrary|SetBlackboardValueasBool (Variables|Default|GetIsAlive) (Variables|/Game/Blueprints/IceGiantAI/IceGiantBoss.IceGiantBoss_C|GetIsAlive _output_get))
  (Class|BTFunctionLibrary|SetBlackboardValueasObject (Variables|Default|GetPitToGoTo) (Variables|/Game/Blueprints/IceGiantAI/IceGiantBoss.IceGiantBoss_C|GetCurrentPit _output_get))
  (Class|BTFunctionLibrary|SetBlackboardValueasObject (Variables|Default|GetPlayer) _returnvalue)
  (Class|BTFunctionLibrary|SetBlackboardValueasObject (Variables|Default|GetCenter) (Variables|/Game/Blueprints/IceGiantAI/IceGiantBoss.IceGiantBoss_C|GetcenterSpot _output_get))
  (Class|BTFunctionLibrary|SetBlackboardValueasFloat (Variables|Default|GetDistance) (Transformation|GetDistanceTo (Variables|Default|GetBos) _returnvalue))
  (bind _asfrost_ai (Utilities|Casting|CastToFrostAi OwnerController))
  (Class|BrainComponent|RestartLogic (Variables|/Script/AIModule.AIController|GetBrainComponent _asfrost_ai)))