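; FireStarter is a one-shot trigger actor that wakes the Ice Giant boss when a character touches it.
; On BeginPlay it caches the first IceGiantBoss found in the level.
; When any Character-derived actor overlaps it, it sets the boss active, turns on gravity for its Box component and destroys itself one second later through its lifespan.
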(event EventBeginPlay
  (bind _outactors (Actor|GetAllActorsOfClass "/Game/Blueprints/IceGiantAI/IceGiantBoss.IceGiantBoss_C"))
  (Variables|Default|Setboss (Utilities|Array|Get(acopy) _outactors)))

(event EventActorBeginOverlap
  (params (OtherActor :type Actor%20Object%20Reference))
  (if (Utilities|ClassIsChildOf (Utilities|GetClass OtherActor) "/Script/Engine.Character")
    (Variables|/Game/Blueprints/IceGiantAI/IceGiantBoss.IceGiantBoss_C|SetIsActive (Variables|Default|Getboss) true)
    (Physics|SetEnableGravity (Variables|Default|GetBox) true)
    (Actor|SetLifeSpan 1.0)))

(event EventTick
  (params (DeltaSeconds :type Float%20%28single-precision%29)))

(fn ConstructionScript)